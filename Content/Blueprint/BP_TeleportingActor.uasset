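; BP_TeleportingActor is an actor that dissolves, teleports between two positions and fades back in when Enter is pressed.
; BeginPlay creates a dynamic dissolve material on the Cube and enables player input on the actor.
; Tick steps the material's Opacity down or up each frame, moving the actor once fully faded out.
; Enter alternates the destination via a FlipFlop and is ignored until the previous fade-in completes.
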(event EventBeginPlay
  (bind _returnvalue (Rendering|Material|CreateDynamicMaterialInstance (Variables|Default|GetCube) 0 "/Game/MyMat/MI_Dissolve.MI_Dissolve" "None" :!class /Script/Engine.PrimitiveComponent))
  (Variables|Default|SetMIDR _returnvalue)
  (Input|EnableInput (Game|GetPlayerController 0)))

(event Collision|EventActorBeginOverlap
  (params (OtherActor :type Actor%20Object%20Reference)))

(event EventTick
  (params (DeltaSeconds :type Float%20%28single-precision%29))
  (bind _returnvalue (Rendering|Material|GetScalarParameterValue (Variables|Default|GetMIDR) "Opacity" :!class /Script/Engine.MaterialInstanceDynamic))
  (if (Variables|Default|GetDissolving)
    (CallFunction|FadeOut _returnvalue)
    (else
      (CallFunction|Fadein _returnvalue))))

(event Input|KeyboardEvents|Enter
  (params (Key :type Key%20Structure :default "None"))
  (:Pressed
    (if (Variables|Default|GetFadeInEnded)
      (Variables|Default|SetDissolving true)
      (Utilities|FlowControl|FlipFlop
        (:A
          (Variables|Default|SetNextPos (Variables|Default|GetPos2)))
        (:B
          (Variables|Default|SetNextPos (Variables|Default|GetPos1))))
      (Variables|Default|SetFadeInEnded false))))

(fn ConstructionScript)

(fn FadeOut
  (params (Opacity :type Float%20%28double-precision%29))
  (if (> Opacity 0.0)
    (Rendering|Material|SetScalarParameterValue (Variables|Default|GetMIDR) "Opacity" (- Opacity 0.01) :!class /Script/Engine.MaterialInstanceDynamic)
    (else
      (Transformation|SetActorLocation (Variables|Default|GetNextPos) false true)
      (Variables|Default|SetDissolving false))))

(fn Fadein
  (params (Opacity :type Float%20%28double-precision%29))
  (if (< Opacity 1.0)
    (Rendering|Material|SetScalarParameterValue (Variables|Default|GetMIDR) "Opacity" (+ Opacity 0.01) :!class /Script/Engine.MaterialInstanceDynamic)
    (else
      (Variables|Default|SetFadeInEnded true))))