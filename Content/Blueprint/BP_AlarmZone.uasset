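; BP_AlarmZone is a trigger zone that raises a visual alarm while the third-person character is inside it.
; Overlap begin and end set the alarm flags and drive wall intensity, wall color and alarm-object color through a Material Parameter Collection, turning yellow on entry and resetting on exit.
; The actor enables player input on BeginPlay, so inside the zone K shows green for a shutdown and L red for a failed one.
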(event EventBeginPlay
  (Input|EnableInput (Game|GetPlayerController 0)))

(event EventTick
  (params (DeltaSeconds :type Float%20%28single-precision%29)))

(event Collision|EventActorBeginOverlap
  (params (OtherActor :type Actor%20Object%20Reference))
  ;[0.15 0.15 0.15 0.5] Caso attivazione allarme
  (Class|KismetSystemLibrary|IsObjectOfSoftClass OtherActor "/Game/ThirdPerson/Blueprints/BP_ThirdPersonCharacter.BP_ThirdPersonCharacter_C"
    (:True
      (Variables|Default|SetInTriggerZone true)
      (Variables|Default|SetAlarmed true)
      (Rendering|Material|SetScalarParameterValue (Variables|Default|GetMPC) (Utilities|Name|MakeLiteralName "WallIntensity") 1e+01 :!class /Script/Engine.KismetMaterialLibrary)
      (Rendering|Material|SetVectorParameterValue (Variables|Default|GetMPC) (Utilities|Name|MakeLiteralName "WallColor") (Utilities|Struct|MakeLinearColor 1.0 1.0 0.0 0.0) :!class /Script/Engine.KismetMaterialLibrary)
      (Rendering|Material|SetVectorParameterValue (Variables|Default|GetMPC) (Utilities|Name|MakeLiteralName "AlarmObjectColor") (Utilities|Struct|MakeLinearColor 1.0 1.0 0.0 0.0) :!class /Script/Engine.KismetMaterialLibrary))))

(event Collision|EventActorEndOverlap
  (params (OtherActor :type Actor%20Object%20Reference))
  ;[0.15 0.15 0.15 0.5] Caso disattivazione allarme
  (Class|KismetSystemLibrary|IsObjectOfSoftClass OtherActor "/Game/ThirdPerson/Blueprints/BP_ThirdPersonCharacter.BP_ThirdPersonCharacter_C"
    (:True
      (Variables|Default|SetInTriggerZone false)
      (Variables|Default|SetAlarmed false)
      (Rendering|Material|SetScalarParameterValue (Variables|Default|GetMPC) (Utilities|Name|MakeLiteralName "WallIntensity") 0.0 :!class /Script/Engine.KismetMaterialLibrary)
      (Rendering|Material|SetVectorParameterValue (Variables|Default|GetMPC) (Utilities|Name|MakeLiteralName "WallColor") (Utilities|Struct|MakeLinearColor 0.0 0.0 0.0 0.0) :!class /Script/Engine.KismetMaterialLibrary)
      (Rendering|Material|SetVectorParameterValue (Variables|Default|GetMPC) (Utilities|Name|MakeLiteralName "AlarmObjectColor") (Utilities|Struct|MakeLinearColor 0.0 0.0 0.0 0.0) :!class /Script/Engine.KismetMaterialLibrary))))

(event Input|KeyboardEvents|K
  (params (Key :type Key%20Structure :default "None"))
  ;[0.15 0.15 0.15 0.5] Caso spegnimento allarme
  (:Pressed
    (if (Variables|Default|GetInTriggerZone)
      (Rendering|Material|SetVectorParameterValue (Variables|Default|GetMPC) (Utilities|Name|MakeLiteralName "WallColor") (Utilities|Struct|MakeLinearColor 0.0 1.0 0.0 0.0) :!class /Script/Engine.KismetMaterialLibrary)
      (Rendering|Material|SetVectorParameterValue (Variables|Default|GetMPC) (Utilities|Name|MakeLiteralName "AlarmObjectColor") (Utilities|Struct|MakeLinearColor 0.0 1.0 0.0 0.0) :!class /Script/Engine.KismetMaterialLibrary))))

(event Input|KeyboardEvents|L
  (params (Key :type Key%20Structure :default "None"))
  ;[0.15 0.15 0.15 0.5] Caso fallimento spegnimento allarme
  (:Pressed
    (if (Variables|Default|GetInTriggerZone)
      (Rendering|Material|SetVectorParameterValue (Variables|Default|GetMPC) (Utilities|Name|MakeLiteralName "WallColor") (Utilities|Struct|MakeLinearColor 1.0 0.0 0.0 0.0) :!class /Script/Engine.KismetMaterialLibrary)
      (Rendering|Material|SetVectorParameterValue (Variables|Default|GetMPC) (Utilities|Name|MakeLiteralName "AlarmObjectColor") (Utilities|Struct|MakeLinearColor 1.0 0.0 0.0 0.0) :!class /Script/Engine.KismetMaterialLibrary))))

(fn ConstructionScript)