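; BP_TimeLapse drives wall material parameters from a directional light's pitch, apparently for a day-night time lapse.
; Each Tick switches WallIntensity in a Material Parameter Collection off for negative pitch, on otherwise.
; It also sets WallColor by lerping amber toward black with the inverse absolute pitch, so the color darkens near the horizon.
; The Blueprint only reads the light's rotation and never changes it.
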(event EventBeginPlay)

(event Collision|EventActorBeginOverlap
  (params (OtherActor :type Actor%20Object%20Reference)))

(event EventTick
  (params (DeltaSeconds :type Float%20%28single-precision%29))
  (bind _directionallight (Variables|Default|GetDirectionalLight))
  (bind _lightcomponent (Variables|/Script/Engine.Light|GetLightComponent _directionallight))
  (bind _returnvalue (Transformation|GetWorldRotation _lightcomponent))
  (bind _pitch (Math|Rotator|BreakRotator _returnvalue))
  (Utilities|FlowControl|Sequence
    (:then_0
      (if (< _pitch 0.0)
        (Rendering|Material|SetScalarParameterValue (Variables|Default|GetMPC) (Utilities|Name|MakeLiteralName "WallIntensity") 0.0 :!class /Script/Engine.KismetMaterialLibrary)
        (else
          (Rendering|Material|SetScalarParameterValue (Variables|Default|GetMPC) (Utilities|Name|MakeLiteralName "WallIntensity") 1.0 :!class /Script/Engine.KismetMaterialLibrary))))
    (:then_1
      (Rendering|Material|SetVectorParameterValue (Variables|Default|GetMPC) (Utilities|Name|MakeLiteralName "WallColor") (Math|Color|Lerp(LinearColor) :A "(R=1.000000,G=0.752520,B=0.000000,A=1.000000)" :Alpha (/ 1.0 (Math|Float|Absolute(Float) _pitch))) :!class /Script/Engine.KismetMaterialLibrary))))

(fn ConstructionScript)