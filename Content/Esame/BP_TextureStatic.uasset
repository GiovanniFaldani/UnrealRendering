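; BP_TextureStatic is an actor whose plane shows a randomly chosen texture, re-rolled on BeginPlay and whenever C is pressed.
; The construction script applies a dynamic instance of M_TextureStatic to the plane.
; RandomizeTexture draws an index from a random stream into the Textures array and sets the material's Texture parameter.
; Its debug print makes a separate stream draw, so the printed index can differ from the applied one.
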(event EventBeginPlay
  (Input|EnableInput (Game|GetPlayerController 0))
  (CallFunction|RandomizeTexture))

(event Collision|EventActorBeginOverlap
  (params (OtherActor :type Actor%20Object%20Reference)))

(event EventTick
  (params (DeltaSeconds :type Float%20%28single-precision%29)))

(event Input|KeyboardEvents|C
  (params (Key :type Key%20Structure :default "None"))
  (:Pressed
    (CallFunction|RandomizeTexture)))

(fn ConstructionScript
  (bind _returnvalue (Rendering|Material|CreateDynamicMaterialInstance "/Game/Esame/M_TextureStatic.M_TextureStatic" "TextureStatic" "None" :!class /Script/Engine.KismetMaterialLibrary))
  (bind _output_get (Variables|Default|SetDynMatRef _returnvalue))
  (Rendering|Material|SetMaterial (Variables|Default|GetPlane) 0 _output_get))

(fn RandomizeTexture
  (bind _randomstream (Variables|Default|GetRandomStream))
  (bind _textures (Variables|Default|GetTextures))
  (bind _returnvalue (Utilities|Array|Length _textures))
  (bind _returnvalue_2 (Class|KismetMathLibrary|RandomIntegerfromStream _randomstream _returnvalue))
  (bind _output_get (Variables|Default|SetTextureIndex _returnvalue_2))
  (Rendering|Material|SetTextureParameterValue (Variables|Default|GetDynMatRef) "Texture" (Utilities|Array|Get(acopy) (Variables|Default|GetTextures) _output_get))
  (Development|PrintString (Utilities|String|Append (Utilities|String|MakeLiteralString "Set texture index to: ") (Utilities|String|ToString(Integer) _returnvalue_2))))